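; BP_Switch is an interactable light switch that toggles the lights referenced by its Lights variable.
; Interact calls the Switch event, which sends a Toggle message to Lights; a SwitchOff message node exists but never runs.
; A Sphere overlap shows the Text component only while the player character is in range.
; The construction script makes the text visible, and BeginPlay hides it.
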(event OnComponentBeginOverlap(Sphere)
  (params (OverlappedComponent :type Primitive%20Component%20Object%20Reference) (OtherActor :type Actor%20Object%20Reference) (OtherComp :type Primitive%20Component%20Object%20Reference) (OtherBodyIndex :type Integer) (bFromSweep :type Boolean) (SweepResult :type Hit%20Result%20Structure%20%28by%20ref%29))
  (if (== OtherActor (Game|GetPlayerCharacter 0))
    (Rendering|SetVisibility (Variables|Default|GetText) true false)))

(event OnComponentEndOverlap(Sphere)
  (params (OverlappedComponent :type Primitive%20Component%20Object%20Reference) (OtherActor :type Actor%20Object%20Reference) (OtherComp :type Primitive%20Component%20Object%20Reference) (OtherBodyIndex :type Integer))
  (if (== OtherActor (Game|GetPlayerCharacter 0))
    (Rendering|SetVisibility (Variables|Default|GetText) false false)))

(event Custom|Switch
  (Class|BPISwitchable|Toggle(Message) (Variables|Default|GetLights)))

(event EventBeginPlay
  (Rendering|SetVisibility (Variables|Default|GetText) false false))

(event EventInteract
  (CallFunction|Switch))

(fn ConstructionScript
  (Rendering|SetVisibility (Variables|Default|GetText) true false))