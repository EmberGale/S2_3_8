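; BP_Light is a switchable light actor that controls the visibility of its PointLight component.
; Switchon and SwitchOff events show or hide the light, and IsOn reports whether it is visible.
; Toggle sets visibility from the inverse of a FlipFlop's state, independent of the light's actual visibility, and prints debug text.
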(event EventSwitchOff
  (Rendering|SetVisibility (Variables|Default|GetPointLight) false false))

(event EventSwitchon
  (Rendering|SetVisibility (Variables|Default|GetPointLight) true false))

(event EventToggle
  (Development|PrintText "Toggle")
  (bind _isa (Utilities|FlowControl|FlipFlop)
    (:A
      _)
    (:B
      _))
  (Rendering|SetVisibility (Variables|Default|GetPointLight) (not _isa) false)
  (Development|PrintText (Utilities|Text|ToText(Boolean) _isa)))

(fn ConstructionScript)

(fn Ison
  (return (Rendering|IsVisible (Variables|Default|GetPointLight))))